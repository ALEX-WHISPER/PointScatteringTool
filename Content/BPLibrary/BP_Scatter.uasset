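; BP_Scatter scatters instanced static meshes from points generated for a referenced actor, apparently exercising scatter helper functions.
; SimpleScatter feeds ScatterActor's points, controlled by intensity and a drop-Z flag, into CreateInstances, which rebuilds the instances at uniform scale.
; NavScatter first converts those points into navmesh points using the level's RecastNavMesh and a tall query extent.
; Separate functions clear instances and print the target's root component bounds.
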(fn `Clear`
  (`InstancedStaticMeshComponent.ClearInstances` (`self.InstancedStaticMesh`)))

(fn `CreateInstances`
  (params (PositionArray :type "Array of Vector Structure"))
  (`InstancedStaticMeshComponent.ClearInstances` (`self.InstancedStaticMesh`))
  (for _array_element PositionArray
    (`InstancedStaticMeshComponent.AddInstance` (`self.InstancedStaticMesh`) (`KismetMathLibrary.MakeTransform` _array_element (struct) (`KismetMathLibrary.Conv_DoubleToVector` (`self.ScatteredPointScale`))) false)))

(fn `Debug Actor Bounds`
  (bind (_outcenter _outextent) (`self.GetRootComponentBounds` (`self.ScatteringActor`)))
  (bind (_outcenter_2 _outextent_2) (`self.GetRootComponentLocalBounds` (`self.ScatteringActor`)))
  (`KismetSystemLibrary.PrintString` (`KismetStringLibrary.Concat_StrStr` (`KismetTextLibrary.Conv_TextToString` (`|FormatText` " \n-----Bounds----- \nCenter: {Center} \nExtent: {Extent} \n" (`KismetStringLibrary.Conv_VectorToString` _outcenter) (`KismetStringLibrary.Conv_VectorToString` _outextent))) (`KismetTextLibrary.Conv_TextToString` (`|FormatText` "-----Local Bounds----- \nCenter: {Center} \nExtent: {Extent} \n" (`KismetStringLibrary.Conv_VectorToString` _outcenter_2) (`KismetStringLibrary.Conv_VectorToString` _outextent_2))))))

(fn `NavScatter`
  (bind _returnvalue (`self.ScatterActor` (`self.ScatteringActor`) (`self.ScatterIntensity`) (`self.bDropZ`)))
  (bind _returnvalue_2 (`GameplayStatics.GetActorOfClass` "/Script/NavigationSystem.RecastNavMesh"))
  (bind _returnvalue_3 (`self.ConvertScatteredPointsIntoNavmeshPoints` _returnvalue _returnvalue_2 (10.0 10.0 1000.0)))
  (`self.CreateInstances` _returnvalue_3))

(fn `SimpleScatter`
  (bind _returnvalue (`self.ScatterActor` (`self.ScatteringActor`) (`self.ScatterIntensity`) (`self.bDropZ`)))
  (`self.CreateInstances` _returnvalue))

(fn `UserConstructionScript`)